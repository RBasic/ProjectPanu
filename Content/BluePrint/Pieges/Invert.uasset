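; Trap actor that temporarily sets the Reverse value of a ThirdPersonCharacterPieges to negative, presumably inverting its controls.
; Overlapping the LePiege component casts the other actor to that character and flips Reverse.
; A fixed two-second Delay then restores it to positive, and overlaps during that wait do not restart the timer.
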(event `self.lePiege.OnComponentBeginOverlap`
  (params (OverlappedComponent :type "PrimitiveComponent Object Reference") (OtherActor :type "Actor Object Reference") (OtherComp :type "PrimitiveComponent Object Reference") (OtherBodyIndex :type Integer) (bFromSweep :type Boolean) (SweepResult :type "HitResult Structure (by ref)"))
  (bind _asthird_person_character_pieges (cast `/Game/BluePrint/ThirdPersonCharacterPieges` OtherActor))
  (set `/Game/BluePrint/ThirdPersonCharacterPieges.reverse` -1.0 _asthird_person_character_pieges)
  (`KismetSystemLibrary.Delay` 2.0)
  (set `/Game/BluePrint/ThirdPersonCharacterPieges.reverse` 1.0 _asthird_person_character_pieges))

(fn `UserConstructionScript`
  (`parent.UserConstructionScript`))