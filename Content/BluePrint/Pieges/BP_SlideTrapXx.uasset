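; BP_SlideTrapXx is a trap Blueprint whose static mesh slides along its local X axis when triggered.
; The ActivateSlideTrap event plays a timeline that drives the mesh's relative X location while keeping its current Y and Z.
; It contains no overlap detection, reset or damage logic, so activation relies on an external call to that event.
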(event `self.ActivateSlideTrap`
  (bind (_relativelocation_x _relativelocation_y _relativelocation_z) (`KismetMathLibrary.BreakVector` (`SceneComponent.RelativeLocation` (`self.StaticMesh`))))
  (bind (_direction _x) (`Timeline|Timeline_0`)
    (:`Update`
      (`SceneComponent.K2_SetRelativeLocation` (`self.StaticMesh`) (`KismetMathLibrary.MakeVector` _x _relativelocation_y _relativelocation_z) false false))))

(fn `UserConstructionScript`
  (`parent.UserConstructionScript`))