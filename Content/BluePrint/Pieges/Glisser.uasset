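; Slip trap actor that temporarily alters the ground friction of a ThirdPersonCharacterPieges entering its LePiege component.
; The overlap plays a timeline that animates the character movement's GroundFriction, then after a delay a second timeline animates it again, presumably restoring grip.
; A never-reset DoOnce precedes the cast, so the first overlap by any actor uses up the trap.
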(event `self.lePiege.OnComponentBeginOverlap`
  (params (OverlappedComponent :type "PrimitiveComponent Object Reference") (OtherActor :type "Actor Object Reference") (OtherComp :type "PrimitiveComponent Object Reference") (OtherBodyIndex :type Integer) (bFromSweep :type Boolean) (SweepResult :type "HitResult Structure (by ref)"))
  (`/Engine/EditorBlueprintResources/StandardMacros.DoOnce` false
    (:`Completed`
      (bind _asthird_person_character_pieges (cast `/Game/BluePrint/ThirdPersonCharacterPieges` OtherActor))
      (bind (_direction _newtrack_0) (`Timeline|Timeline_0`)
        (:`Update`
          (bind _charactermovement (`Character.CharacterMovement` _asthird_person_character_pieges))
          (set `CharacterMovementComponent.GroundFriction` _newtrack_0 _charactermovement))
        (:`Finished`
          (`KismetSystemLibrary.Delay` 5.0)
          (bind (_direction_2 _newtrack_0_2) (`Timeline|Timeline_1`)
            (:`Update`
              (set `CharacterMovementComponent.GroundFriction` _newtrack_0_2 _charactermovement))))))))

(fn `UserConstructionScript`
  (`parent.UserConstructionScript`))