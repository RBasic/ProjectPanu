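; BP_Lamp_Rectangular is a rect light lamp that blinks on and off, with randomized brightness and blink interval.
; The construction script picks a random intensity for RectLight and an initial random blink delay within set min/max ranges.
; BeginPlay starts a looping timer that toggles the light's visibility.
; Each blink re-rolls the delay variable, but the timer is never reset, so its period stays constant.
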(event `self.ReceiveBeginPlay`
  (`KismetSystemLibrary.K2_SetTimerDelegate` (delegate `BlinkingLight`) (`self.randomChosen`) true))

(event `BlinkingLight`
  (`SceneComponent.ToggleVisibility` (`self.RectLight`) true)
  (set `self.randomChosen` (`KismetMathLibrary.RandomFloatInRange` (`self.minFloatBlink`) (`self.maxFloatBlink`))))

(fn `UserConstructionScript`
  ;[1 1 1] Permet de set les PointLights (intensités et temps avant les blinks)
  (bind _output_get (set `self.globalIntensity` (`KismetMathLibrary.RandomFloatInRange` (`self.minFloatIntensity`) (`self.maxFloatIntensity`))))
  (`LightComponent.SetIntensity` (`self.RectLight`) _output_get)
  (set `self.randomChosen` (`KismetMathLibrary.RandomFloatInRange` (`self.minFloatBlink`) (`self.maxFloatBlink`))))