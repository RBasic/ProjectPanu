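; BP_Lamp_Constant is a lamp Blueprint that gives its five point lights a shared, randomized brightness.
; The Construction Script rolls GlobalIntensity between MinFloatIntensity and MaxFloatIntensity, gathers the point lights into BasementLights and applies that value to each.
; The roll uses no seed, so the intensity can change whenever construction reruns, and this graph contains no runtime flicker or update logic.
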(fn `UserConstructionScript`
  ;[1 1 1] Permet de set les PointLights (intensités des lampes)
  (bind _output_get (set `self.globalIntensity` (`KismetMathLibrary.RandomFloatInRange` (`self.minFloatIntensity`) (`self.maxFloatIntensity`))))
  (bind _output_get_2 (set `self.basementLights` (`|MakeArray` (`self.PointLight`) (`self.PointLight1`) (`self.PointLight2`) (`self.PointLight3`) (`self.PointLight4`))))
  (for _array_element _output_get_2
    (`LightComponent.SetIntensity` _array_element _output_get)))