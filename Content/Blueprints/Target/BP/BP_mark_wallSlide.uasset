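; BP_mark_wallSlide is a shootable target that triggers a sliding wall trap.
; When a FirstPersonProjectile overlaps its Box, a DoOnce starts a timeline that animates the static mesh's relative roll.
; When the timeline finishes, it calls TrapSlideWall on the referenced Piege and destroys the Box, so the target works only once.
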(event `self.ReceiveBeginPlay`)

(event `self.Box.OnComponentBeginOverlap`
  (params (OverlappedComponent :type "PrimitiveComponent Object Reference") (OtherActor :type "Actor Object Reference") (OtherComp :type "PrimitiveComponent Object Reference") (OtherBodyIndex :type Integer) (bFromSweep :type Boolean) (SweepResult :type "HitResult Structure (by ref)"))
  (bind (_relativerotation_roll _relativerotation_pitch _relativerotation_yaw) (`KismetMathLibrary.BreakRotator` (`SceneComponent.RelativeRotation` (`self.StaticMeshComponent`))))
  (cast `/Game/Blueprints/FirstPersonProjectile` OtherActor)
  (`/Engine/EditorBlueprintResources/StandardMacros.DoOnce` false
    (:`Completed`
      (bind (_direction _x) (`Timeline|Timeline_0` :!via `PlayFromStart`)
        (:`Update`
          (`SceneComponent.K2_SetRelativeRotation` (`self.StaticMeshComponent`) (`KismetMathLibrary.MakeRotator` _x _relativerotation_pitch _relativerotation_yaw) false false))
        (:`Finished`
          (`/Game/Blueprints/Pieges/BPP_SlideTrap.Trap Slide Wall` (`self.Piege`))
          (`ActorComponent.K2_DestroyComponent` (`self.Box`)))))))

(fn `UserConstructionScript`)