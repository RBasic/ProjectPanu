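; Spotlight Blueprint that blinks with a neon sound effect.
; The construction script randomizes the light's intensity and picks a random interval for a looping timer started at BeginPlay.
; Each timer tick drives a FlipFlop that plays the sound, toggles the spotlight's visibility and flips a flag.
; When that flag is false, a further random delay precedes the toggle, making the blink uneven.
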(event `self.ReceiveBeginPlay`
  (`KismetSystemLibrary.K2_SetTimerDelegate` (delegate `BlinkingLight`) (`self.Random`) true))

(event `BlinkingLight`
  (if (not (`self.Toogled`))
    (`KismetSystemLibrary.Delay` (`KismetMathLibrary.RandomFloatInRange` (`self.Min`) (`self.Max`))))
  (`/Engine/EditorBlueprintResources/StandardMacros.FlipFlop`
    (:`A`
      (`GameplayStatics.PlaySound2D` "/Game/Sounds/AMB/Sound_Cue/Neon.Neon" 1.0 1.0 0.0 null null)
      (`SceneComponent.ToggleVisibility` (`self.SpotLightComponent`) false)
      (set `self.Toogled` true))
    (:`B`
      (`GameplayStatics.PlaySound2D` "/Game/Sounds/AMB/Sound_Cue/Neon.Neon" 1.0 1.0 0.0 null null)
      (`SceneComponent.ToggleVisibility` (`self.SpotLightComponent`) false)
      (set `self.Toogled` false))))

(fn `UserConstructionScript`
  (`LightComponent.SetIntensity` (`self.SpotLightComponent`) (`KismetMathLibrary.RandomFloatInRange` (`self.MinInt`) (`self.MaxInt`)))
  (set `self.Random` (`KismetMathLibrary.RandomFloatInRange` (`self.Min`) (`self.Max`))))