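; BP_BasementLight is a basement spotlight that flickers on and off at irregular intervals.
; The construction script gives the spotlight a random intensity within a configurable range, so placed lights can differ in brightness.
; The BlinkingLights event runs an endless loop that waits a random retriggerable delay between configurable bounds, then toggles the spotlight's visibility.
; Nothing in these graphs calls BlinkingLights.
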(event `Blinking Lights`
  (`KismetSystemLibrary.RetriggerableDelay` (`KismetMathLibrary.RandomFloatInRange` (`self.minFloatBlink`) (`self.maxFloatBlink`)) :!label _label)
  (`SceneComponent.ToggleVisibility` (`self.SpotLightComponent`) false)
  (goto _label))

(fn `UserConstructionScript`
  (`LightComponent.SetIntensity` (`self.SpotLightComponent`) (`KismetMathLibrary.RandomFloatInRange` (`self.minFloatIntensity`) (`self.maxFloatIntensity`))))