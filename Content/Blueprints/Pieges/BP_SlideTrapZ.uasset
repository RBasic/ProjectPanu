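; BP_SlideTrapZ is a trap piece that slides its static mesh along the relative Z axis.
; The TrapSlideWall event plays the TL_SlideZ timeline, which writes its Z value to the mesh's relative location each update, keeping X and Y.
; An ActivateTrapSlide function applies the same Z move from a passed-in value, but the event graph does not call it.
; The construction script only runs the parent's.
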(event `self.Trap Slide Wall`
  (bind (_relativelocation_x _relativelocation_y) (`KismetMathLibrary.BreakVector` (`SceneComponent.RelativeLocation` (`self.StaticMesh`))))
  (bind (_direction _z) (`Timeline|TL_SlideZ`)
    (:`Update`
      (`SceneComponent.K2_SetRelativeLocation` (`self.StaticMesh`) (`KismetMathLibrary.MakeVector` _relativelocation_x _relativelocation_y _z) false false))))

(fn `Activate Trap Slide`
  (params (TimeLine :type "Float (double-precision)" :default 0.0))
  (bind (_relativelocation_x _relativelocation_y) (`KismetMathLibrary.BreakVector` (`SceneComponent.RelativeLocation` (`self.StaticMesh`))))
  (`SceneComponent.K2_SetRelativeLocation` (`self.StaticMesh`) (`KismetMathLibrary.MakeVector` _relativelocation_x _relativelocation_y TimeLine) false false))

(fn `UserConstructionScript`
  (`parent.UserConstructionScript`))