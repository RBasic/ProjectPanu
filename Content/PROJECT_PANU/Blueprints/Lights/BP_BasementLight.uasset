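; BP_BasementLight is a basement spotlight that blinks on and off, with randomized brightness and blink rate.
; The construction script picks a random intensity and blink interval within configurable ranges.
; BeginPlay starts a looping timer that toggles the spotlight's visibility.
; Each blink re-rolls the interval variable, but the timer is never reset, so it keeps the period it started with.
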(event `self.ReceiveBeginPlay`
  (`KismetSystemLibrary.K2_SetTimerDelegate` (delegate `BlinkingLight`) (`self.randomChosen`) true))

(event `BlinkingLight`
  (`SceneComponent.ToggleVisibility` (`self.SpotLightComponent`) false)
  (set `self.randomChosen` (`KismetMathLibrary.RandomFloatInRange` (`self.minFloatBlink`) (`self.maxFloatBlink`))))

(fn `UserConstructionScript`
  (`LightComponent.SetIntensity` (`self.SpotLightComponent`) (`KismetMathLibrary.RandomFloatInRange` (`self.minFloatIntensity`) (`self.maxFloatIntensity`)))
  (set `self.randomChosen` (`KismetMathLibrary.RandomFloatInRange` (`self.minFloatBlink`) (`self.maxFloatBlink`))))