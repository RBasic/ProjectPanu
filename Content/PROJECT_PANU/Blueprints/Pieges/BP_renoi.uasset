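; Trap actor that drives a temporary screen or material effect when something overlaps its LePiege component.
; On overlap, two timelines animate the "radius" and "zooom" scalars in the Param material parameter collection.
; Each timeline waits briefly after finishing, then reverses through a DoOnce that is never reset, so the automatic reversal happens only once per instance.
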(event `self.lePiege.OnComponentBeginOverlap`
  (params (OverlappedComponent :type "PrimitiveComponent Object Reference") (OtherActor :type "Actor Object Reference") (OtherComp :type "PrimitiveComponent Object Reference") (OtherBodyIndex :type Integer) (bFromSweep :type Boolean) (SweepResult :type "HitResult Structure (by ref)"))
  (`|ExecutionSequence`
    (:`then_0`
      (bind (_direction _newtrack_0) (`Timeline|Timeline_0` :!via `PlayFromStart` :!label _label)
        (:`Update`
          (`KismetMaterialLibrary.SetScalarParameterValue` "/Game/PROJECT_PANU/Blueprints/PostProcess/param.param" "radius" _newtrack_0))
        (:`Finished`
          (`KismetSystemLibrary.Delay` 2.0)
          (`/Engine/EditorBlueprintResources/StandardMacros.DoOnce` false
            (:`Completed`
              (goto _label :!via `ReverseFromEnd`))))))
    (:`then_1`
      (bind (_direction_2 _newtrack_0_2) (`Timeline|Timeline_1` :!label _label_2)
        (:`Update`
          (`KismetMaterialLibrary.SetScalarParameterValue` "/Game/PROJECT_PANU/Blueprints/PostProcess/param.param" "zooom" _newtrack_0_2))
        (:`Finished`
          (`KismetSystemLibrary.Delay` 2.0)
          (`/Engine/EditorBlueprintResources/StandardMacros.DoOnce` false
            (:`Completed`
              (goto _label_2 :!via `ReverseFromEnd`))))))))

(fn `UserConstructionScript`
  (`parent.UserConstructionScript`))