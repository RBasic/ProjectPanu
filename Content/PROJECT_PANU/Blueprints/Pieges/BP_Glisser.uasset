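; BP_Glisser is a one-shot trap that temporarily alters a character's ground friction, named for slipping.
; Overlapping LePiege plays a 2D sound each time, while a DoOnce ahead of the ThirdPersonCharacter cast lets only the first overlap through.
; It calls DegeuEffect and drives GroundFriction with a timeline.
; After a delay, it calls UnDegeuEffect, runs a second friction timeline, then destroys itself.
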(event `self.lePiege.OnComponentBeginOverlap`
  (params (OverlappedComponent :type "PrimitiveComponent Object Reference") (OtherActor :type "Actor Object Reference") (OtherComp :type "PrimitiveComponent Object Reference") (OtherBodyIndex :type Integer) (bFromSweep :type Boolean) (SweepResult :type "HitResult Structure (by ref)"))
  (`GameplayStatics.PlaySound2D` null 1.0 1.0 0.0 null null)
  (`/Engine/EditorBlueprintResources/StandardMacros.DoOnce` false
    (:`Completed`
      (bind _asthird_person_character (cast `/Game/PROJECT_PANU/SciFi_Robot/ThirdPersonBP/Blueprints/ThirdPersonCharacter` OtherActor))
      (`|ExecutionSequence`
        (:`then_0`
          (`/Game/PROJECT_PANU/SciFi_Robot/ThirdPersonBP/Blueprints/ThirdPersonCharacter.DegeuEffect` _asthird_person_character))
        (:`then_1`
          (bind (_direction _newtrack_0) (`Timeline|Timeline_0`)
            (:`Update`
              (bind _charactermovement (`Character.CharacterMovement` _asthird_person_character))
              (set `CharacterMovementComponent.GroundFriction` _newtrack_0 _charactermovement))
            (:`Finished`
              (`KismetSystemLibrary.Delay` 5.0)
              (`|ExecutionSequence`
                (:`then_0`
                  (`/Game/PROJECT_PANU/SciFi_Robot/ThirdPersonBP/Blueprints/ThirdPersonCharacter.unDegeuEffect` _asthird_person_character))
                (:`then_1`
                  (bind (_direction_2 _newtrack_0_2) (`Timeline|Timeline_1`)
                    (:`Update`
                      (set `CharacterMovementComponent.GroundFriction` _newtrack_0_2 _charactermovement))
                    (:`Finished`
                      (`self.K2_DestroyActor`))))))))))))

(fn `UserConstructionScript`
  (`parent.UserConstructionScript`))