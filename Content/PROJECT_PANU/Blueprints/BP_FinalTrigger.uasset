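; BP_FinalTrigger is an end-of-game trigger that activates the final doors and then ends the game.
; At BeginPlay it caches every BP_FinalDoors actor in the level.
; When a ThirdPersonCharacter overlaps TriggerDoorAndFinal, it calls ActivateDoors on each door.
; A delay inside that loop leads to GameOver on player 0 a few seconds later, cast to FirstPersonCharacter, unlike the overlap check.
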(event `self.ReceiveBeginPlay`
  (bind _outactors (`GameplayStatics.GetAllActorsOfClass` "/Game/PROJECT_PANU/Blueprints/Building/BP_FinalDoors.BP_FinalDoors_C"))
  (set `self.AllDoors` _outactors))

(event `self.TriggerDoorAndFinal.OnComponentBeginOverlap`
  (params (OverlappedComponent :type "PrimitiveComponent Object Reference") (OtherActor :type "Actor Object Reference") (OtherComp :type "PrimitiveComponent Object Reference") (OtherBodyIndex :type Integer) (bFromSweep :type Boolean) (SweepResult :type "HitResult Structure (by ref)"))
  (cast `/Game/PROJECT_PANU/SciFi_Robot/ThirdPersonBP/Blueprints/ThirdPersonCharacter` OtherActor)
  (for _array_element (`self.AllDoors`)
    (`/Game/PROJECT_PANU/Blueprints/Building/BP_FinalDoors.Activate Doors` _array_element)
    (`KismetSystemLibrary.Delay` 4.0)
    (`/Game/FirstPersonBP/Blueprints/FirstPersonCharacter.GameOver` (cast `/Game/FirstPersonBP/Blueprints/FirstPersonCharacter` (`GameplayStatics.GetPlayerCharacter` 0) :!pure true))))

(fn `UserConstructionScript`)